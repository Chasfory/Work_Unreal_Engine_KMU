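; BP_Door is a door actor that slides upward once two pressure plates are active.
; OpenDoor and CloseDoor events increment and decrement a plate counter, likely called by plate actors.
; Reaching exactly two plays a timeline that lerps the door mesh's relative Z to raise it.
; Any other count on OpenDoor, and every CloseDoor call, reverses the timeline.
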(event Custom|OpenDoor
  (Variables|Default|Setn_plates_activated (+ (Variables|Default|Getn_plates_activated) 1))
  (if (== (Variables|Default|Getn_plates_activated) 2)
    (bind _position (Timeline|Timeline Play)
      (:Update
        (Transformation|SetRelativeLocation (Variables|Default|GetDoor) (Math|Vector|MakeVector 0.0 0.0 (Math|Float|Lerp 1e+02 3e+02 _position)) false false)))
    (else
      (Timeline|Timeline Reverse))))

(event Custom|CloseDoor
  (Variables|Default|Setn_plates_activated (- (Variables|Default|Getn_plates_activated) 1))
  (bind _position (Timeline|Timeline Reverse)
    (:Update
      (Transformation|SetRelativeLocation (Variables|Default|GetDoor) (Math|Vector|MakeVector 0.0 0.0 (Math|Float|Lerp 1e+02 3e+02 _position)) false false))))

(event EventBeginPlay)

(event Collision|EventActorBeginOverlap
  (params (OtherActor :type Actor%20Object%20Reference)))

(event EventTick
  (params (DeltaSeconds :type Float%20%28single-precision%29)))

(fn ConstructionScript)